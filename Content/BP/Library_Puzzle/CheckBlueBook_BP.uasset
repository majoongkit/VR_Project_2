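; Library puzzle trigger that detects Bluebook actors and tracks their count on the player's VRPawnPhysics.
; On begin overlap it destroys the book, increments and prints the count, and spawns a Bluebook_spawn at the collision component's transform.
; On end overlap it decrements and prints the count.
; Each overlap path has its own DoOnce that resets after a short delay to debounce repeat triggers.
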(event OnComponentBeginOverlap(CollisionComponent)
  (params (OverlappedComponent :type Primitive%20Component%20Object%20Reference) (OtherActor :type Actor%20Object%20Reference) (OtherComp :type Primitive%20Component%20Object%20Reference) (OtherBodyIndex :type Integer) (bFromSweep :type Boolean) (SweepResult :type Hit%20Result%20Structure%20%28by%20ref%29))
  (bind _as_vrpawn_physics (Variables|Default|GetAs%20VRPawn%20Physics))
  ;[0.437 0.5609 1] Checktrigger
  (bind _asbluebook (Utilities|Casting|CastToBluebook OtherActor))
  (Utilities|FlowControl|DoOnce false :!label _label
    (:Completed
      (Actor|DestroyActor _asbluebook)
      (bind _output_get (Variables|/Game/VRTemplate/Blueprints/VRPawnPhysics.VRPawnPhysics_C|SetBluebook _as_vrpawn_physics (+ (Variables|/Game/VRTemplate/Blueprints/VRPawnPhysics.VRPawnPhysics_C|GetBluebook _as_vrpawn_physics) 1)))
      (Development|PrintString (Utilities|String|ToString(Integer) _output_get))
      (Game|SpawnActorfromClass "/Game/BP/Library_Puzzle/Bluebook_spawn.Bluebook_spawn_C" (Transformation|GetWorldTransform (Variables|Default|GetCollisionComponent)) "Undefined" "MultiplyWithRoot" 0 0)
      (Utilities|FlowControl|Delay 2.0)
      (goto _label Reset))))

(event OnComponentEndOverlap(CollisionComponent)
  (params (OverlappedComponent :type Primitive%20Component%20Object%20Reference) (OtherActor :type Actor%20Object%20Reference) (OtherComp :type Primitive%20Component%20Object%20Reference) (OtherBodyIndex :type Integer))
  (bind _as_vrpawn_physics (Variables|Default|GetAs%20VRPawn%20Physics))
  ;[0.437 0.5609 1] Checktrigger
  (Utilities|Casting|CastToBluebook OtherActor)
  (Utilities|FlowControl|DoOnce false :!label _label
    (:Completed
      (bind _output_get (Variables|/Game/VRTemplate/Blueprints/VRPawnPhysics.VRPawnPhysics_C|SetBluebook _as_vrpawn_physics (- (Variables|/Game/VRTemplate/Blueprints/VRPawnPhysics.VRPawnPhysics_C|GetBluebook _as_vrpawn_physics) 1)))
      (Development|PrintString (Utilities|String|ToString(Integer) _output_get))
      (Utilities|FlowControl|Delay 2.0)
      (goto _label Reset))))

(event EventBeginPlay
  (bind _asvrpawn_physics (Utilities|Casting|CastToVRPawnPhysics (Game|GetPlayerCharacter 0)))
  (Variables|Default|SetAs%20VRPawn%20Physics _asvrpawn_physics))

(event Collision|EventActorBeginOverlap
  (params (OtherActor :type Actor%20Object%20Reference)))

(event EventTick
  (params (DeltaSeconds :type Float%20%28single-precision%29)))

(fn ConstructionScript)