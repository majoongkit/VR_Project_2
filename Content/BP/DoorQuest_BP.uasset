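; A quest door Blueprint that unlocks and swings open when a Key actor overlaps its Box.
; The overlap shows the door's own Key component, spins it via the SpinKey timeline and destroys it after a delay.
; It also destroys the overlapping Key actor, plays an unlock sound, then after a delay plays the opening sound and rotates Door with the Open timeline.
; A testkey event enters the same sequence directly.
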(event OnComponentBeginOverlap(Box)
  (params (OverlappedComponent :type Primitive%20Component%20Object%20Reference) (OtherActor :type Actor%20Object%20Reference) (OtherComp :type Primitive%20Component%20Object%20Reference) (OtherBodyIndex :type Integer) (bFromSweep :type Boolean) (SweepResult :type Hit%20Result%20Structure%20%28by%20ref%29))
  (bind _key (Variables|Default|GetKey))
  (bind _askey (Utilities|Casting|CastToKey OtherActor))
  (Utilities|FlowControl|Sequence
    (:then_0
      (Rendering|SetVisibility _key true false)
      (bind _spinkey (Timeline|SpinKey Play)
        (:Update
          (Transformation|SetRelativeRotation _key (Math|Rotator|MakeRotator 9e+01 _spinkey 0.0) false false)
          (Utilities|FlowControl|Delay 2.0)
          (Components|DestroyComponent (Variables|Default|GetKey)))))
    (:then_1
      (Actor|DestroyActor _askey)
      (Audio|PlaySound2D "/Game/Sound/DoorKeyUnlock_Cue.DoorKeyUnlock_Cue" 1.0 1.0 0.0 0 0)
      (Utilities|FlowControl|Delay 2.0)
      (Audio|PlaySound2D "/Game/Sound/Open-Door-Store-room_Cue.Open-Door-Store-room_Cue" 1.0 1.0 0.0 0 0)
      (bind _doorrotate (Timeline|open Play)
        (:Update
          (Transformation|SetRelativeRotation (Variables|Default|GetDoor) (Math|Rotator|MakeRotator 0.0 0.0 _doorrotate) false false))))))

(event Custom|test%20key
  (bind _key (Variables|Default|GetKey))
  (Utilities|FlowControl|Sequence
    (:then_0
      (Rendering|SetVisibility _key true false)
      (bind _spinkey (Timeline|SpinKey Play)
        (:Update
          (Transformation|SetRelativeRotation _key (Math|Rotator|MakeRotator 9e+01 _spinkey 0.0) false false)
          (Utilities|FlowControl|Delay 2.0)
          (Components|DestroyComponent (Variables|Default|GetKey)))))
    (:then_1
      (Actor|DestroyActor (stale OnComponentBeginOverlap(Box) _askey))
      (Audio|PlaySound2D "/Game/Sound/DoorKeyUnlock_Cue.DoorKeyUnlock_Cue" 1.0 1.0 0.0 0 0)
      (Utilities|FlowControl|Delay 2.0)
      (Audio|PlaySound2D "/Game/Sound/Open-Door-Store-room_Cue.Open-Door-Store-room_Cue" 1.0 1.0 0.0 0 0)
      (bind _doorrotate (Timeline|open Play)
        (:Update
          (Transformation|SetRelativeRotation (Variables|Default|GetDoor) (Math|Rotator|MakeRotator 0.0 0.0 _doorrotate) false false))))))

(event EventBeginPlay)

(event Collision|EventActorBeginOverlap
  (params (OtherActor :type Actor%20Object%20Reference)))

(event EventTick
  (params (DeltaSeconds :type Float%20%28single-precision%29)))

(fn ConstructionScript)