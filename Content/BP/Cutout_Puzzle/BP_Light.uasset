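; BP_Light is a point light actor, apparently part of the cutout puzzle.
; The construction script sets the PointLight's visibility from the LightIsOn flag.
; The Tocutout event flips LightIsOn, then always hides the light regardless of that flag and sets its color to NewLight.
; BeginPlay, overlap and Tick are unused.
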(event EventBeginPlay)

(event Collision|EventActorBeginOverlap
  (params (OtherActor :type Actor%20Object%20Reference)))

(event EventTick
  (params (DeltaSeconds :type Float%20%28single-precision%29)))

(event EventTocutout
  ;[1 0.8903 0.3585] Set lighting
  (Variables|Default|SetLightIsOn? (not (Variables|Default|GetLightIsOn?)))
  (Rendering|SetVisibility (Variables|Default|GetPointLight) false false)
  (Rendering|Components|Light|SetLightColor (Variables|Default|GetPointLight) (Variables|Default|GetNewLight) true))

(fn ConstructionScript
  (Rendering|SetVisibility (Variables|Default|GetPointLight) (Variables|Default|GetLightIsOn?) false))