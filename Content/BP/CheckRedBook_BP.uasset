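; Trigger actor that tracks Redbook actors entering and leaving its collision component, keeping the count on the player's VRPawn.
; On BeginPlay it caches the player character as a VRPawn.
; Begin overlap with a Redbook increments the pawn's Redbook counter and end overlap decrements it, printing the new value each time.
; Each direction has its own DoOnce that resets after a short delay, debouncing repeated overlaps.
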(event OnComponentBeginOverlap(CollisionComponent)
  (params (OverlappedComponent :type Primitive%20Component%20Object%20Reference) (OtherActor :type Actor%20Object%20Reference) (OtherComp :type Primitive%20Component%20Object%20Reference) (OtherBodyIndex :type Integer) (bFromSweep :type Boolean) (SweepResult :type Hit%20Result%20Structure%20%28by%20ref%29))
  (bind _as_vrpawn (Variables|Default|GetAs%20VRPawn))
  ;[1 0.1865 0.1865] Checktrigger
  (Utilities|Casting|CastToRedbook OtherActor)
  (Utilities|FlowControl|DoOnce false :!label _label
    (:Completed
      (bind _output_get (Variables|/Game/VRTemplate/Blueprints/VRPawn.VRPawn_C|SetRedbook _as_vrpawn (+ (Variables|/Game/VRTemplate/Blueprints/VRPawn.VRPawn_C|GetRedbook _as_vrpawn) 1)))
      (Development|PrintString (Utilities|String|ToString(Integer) _output_get))
      (Utilities|FlowControl|Delay 2.0)
      (goto _label Reset))))

(event OnComponentEndOverlap(CollisionComponent)
  (params (OverlappedComponent :type Primitive%20Component%20Object%20Reference) (OtherActor :type Actor%20Object%20Reference) (OtherComp :type Primitive%20Component%20Object%20Reference) (OtherBodyIndex :type Integer))
  (bind _as_vrpawn (Variables|Default|GetAs%20VRPawn))
  ;[1 0.1865 0.1865] Checktrigger
  (Utilities|Casting|CastToRedbook OtherActor)
  (Utilities|FlowControl|DoOnce false :!label _label
    (:Completed
      (bind _output_get (Variables|/Game/VRTemplate/Blueprints/VRPawn.VRPawn_C|SetRedbook _as_vrpawn (- (Variables|/Game/VRTemplate/Blueprints/VRPawn.VRPawn_C|GetRedbook _as_vrpawn) 1)))
      (Development|PrintString (Utilities|String|ToString(Integer) _output_get))
      (Utilities|FlowControl|Delay 2.0)
      (goto _label Reset))))

(event EventBeginPlay
  (bind _asvrpawn (Utilities|Casting|CastToVRPawn (Game|GetPlayerCharacter 0)))
  (Variables|Default|SetAs%20VRPawn _asvrpawn))

(event Collision|EventActorBeginOverlap
  (params (OtherActor :type Actor%20Object%20Reference)))

(event EventTick
  (params (DeltaSeconds :type Float%20%28single-precision%29)))

(fn ConstructionScript)