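; Fuse box actor for a fuse puzzle, with a hinged door that a motion controller can grab and swing open.
; Grab stores the controller and plays an opening sound if it is within the handle sphere's radius; Release clears it.
; While held, Tick sets the door's world yaw from a look-at between hand and door, clamped to a quarter turn.
; When free, a nearly closed door snaps shut.
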(event EventBeginPlay)

(event Collision|EventActorBeginOverlap
  (params (OtherActor :type Actor%20Object%20Reference)))

(event EventTick
  (params (DeltaSeconds :type Float%20%28single-precision%29))
  (bind _hand (Variables|Default|GetHand))
  (bind _door (Variables|Default|GetDoor))
  (Utilities|IsValid _hand
    (:Is%20Valid
      (Transformation|SetWorldRotation _door (Math|Rotator|MakeRotator 0.0 0.0 (Math|Float|ClampAngle (- (.yaw (Math|Rotator|FindLookatRotation (Transformation|GetWorldLocation _hand) (Transformation|GetWorldLocation _door))) 0.0) -9e+01 0.0)) false false))
    (:Is%20Not%20Valid
      (if (Math|Float|NearlyEqual(Float) (.yaw (Transformation|GetWorldRotation _door)) 0.0 1e+01)
        (Transformation|SetWorldRotation _door "0, 0, 0" false false)))))

(event EventGrab
  (params (Motioncontroll :type Motion%20Controller%20Component%20Object%20Reference))
  (bind _sphere (Variables|Default|GetSphere))
  (if (Utilities|Operators|EqualEqual (Transformation|GetWorldLocation Motioncontroll) (Transformation|GetWorldLocation _sphere) (Variables|/Script/Engine.SphereComponent|GetSphereRadius _sphere))
    (Variables|Default|SetHand Motioncontroll)
    (Audio|PlaySound2D "/Game/Sound/Open_Boxfuse_Cue.Open_Boxfuse_Cue" 1.0 1.0 0.0 0 0)))

(event EventRelease
  (params (Motioncontroll :type Motion%20Controller%20Component%20Object%20Reference))
  (if (== Motioncontroll (Variables|Default|GetHand))
    (Variables|Default|SetHand 0)))

(fn ConstructionScript)