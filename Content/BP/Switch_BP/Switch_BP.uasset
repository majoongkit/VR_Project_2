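; Switch actor that lets a VR player toggle the Light_BP actors sharing its light index.
; BeginPlay gathers every Light_BP in the level.
; A box overlap with VRPawnPhysics enables input and opens a Gate, and leaving disables input and closes it.
; While the Gate is open, either left or right interact input calls ToggleLightMessage on each light with a matching index.
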(event OnComponentBeginOverlap(Box)
  (params (OverlappedComponent :type Primitive%20Component%20Object%20Reference) (OtherActor :type Actor%20Object%20Reference) (OtherComp :type Primitive%20Component%20Object%20Reference) (OtherBodyIndex :type Integer) (bFromSweep :type Boolean) (SweepResult :type Hit%20Result%20Structure%20%28by%20ref%29))
  ;[0 1 0.8065] get array light and interact
  (Utilities|Casting|CastToVRPawnPhysics OtherActor)
  (Input|EnableInput (Game|GetPlayerController 0))
  (Utilities|FlowControl|Gate true) ; enters at Open
)

(event OnComponentEndOverlap(Box)
  (params (OverlappedComponent :type Primitive%20Component%20Object%20Reference) (OtherActor :type Actor%20Object%20Reference) (OtherComp :type Primitive%20Component%20Object%20Reference) (OtherBodyIndex :type Integer))
  ;[0 1 0.8065] get array light and interact
  (Utilities|Casting|CastToVRPawnPhysics OtherActor)
  (Input|DisableInput (Game|GetPlayerController 0))
  (Utilities|FlowControl|Gate true) ; enters at Close
)

(event Input|EnhancedActionEvents|EnhancedInputActionIA_InteractLeft
  (params (ActionValue :type Boolean) (ElapsedSeconds :type Float%20%28double-precision%29) (TriggeredSeconds :type Float%20%28double-precision%29) (InputAction :type Input%20Action%20Object%20Reference :default "/Game/InputAction/IA_InteractLeft.IA_InteractLeft"))
  ;[0 1 0.8065] get array light and interact
  (:Started
    (Utilities|FlowControl|Gate true
      (:Exit
        (for _array_element (Variables|Default|GetOut%20Actors)
          (if (== (Variables|/Game/BP/Switch_BP/Light_BP.Light_BP_C|GetLight%20Index _array_element) (Variables|Default|GetLight%20Idex))
            (Class|BPILight|ToggleLight(Message) _array_element)))))))

(event Input|EnhancedActionEvents|EnhancedInputActionIA_InteractRight
  (params (ActionValue :type Boolean) (ElapsedSeconds :type Float%20%28double-precision%29) (TriggeredSeconds :type Float%20%28double-precision%29) (InputAction :type Input%20Action%20Object%20Reference :default "/Game/InputAction/IA_InteractRight.IA_InteractRight"))
  ;[0 1 0.8065] get array light and interact
  (:Started
    (Utilities|FlowControl|Gate true
      (:Exit
        (for _array_element (Variables|Default|GetOut%20Actors)
          (if (== (Variables|/Game/BP/Switch_BP/Light_BP.Light_BP_C|GetLight%20Index _array_element) (Variables|Default|GetLight%20Idex))
            (Class|BPILight|ToggleLight(Message) _array_element)))))))

(event EventBeginPlay
  (bind _outactors (Actor|GetAllActorsOfClass "/Game/BP/Switch_BP/Light_BP.Light_BP_C"))
  (bind _output_get (Variables|Default|SetOut%20Actors _outactors))
  (for _array_element _output_get
    (Utilities|Array|Add (Utilities|Array|MakeArray _array_element) 0)))

(event Collision|EventActorBeginOverlap
  (params (OtherActor :type Actor%20Object%20Reference)))

(event EventTick
  (params (DeltaSeconds :type Float%20%28single-precision%29)))

(fn ConstructionScript)